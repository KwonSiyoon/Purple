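; Blueprint actor that spawns a trail of NS_22_PowerSmash_1_Ice Niagara effects along its forward vector.
; IceSpawnEvent runs a delayed loop, placing each system a fixed distance further out at a configurable interval until SpawnNum is passed.
; The last few spawns scale up progressively so the trail ends in larger ice bursts.
; Camera shake calls are present but unconnected, so they never run.
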(event Custom|IceSpawnEvent
  (bind _spawnnum (Variables|Default|GetSpawnNum))
  (Variables|Default|SetIsSpawnNum 0)
  (if (<= (Variables|Default|GetIsSpawnNum) _spawnnum) :!label _label
    (Niagara|SpawnSystematLocation "/Game/FightingNiagaraVFX/Niagara/NiagaraSystem/FightingNiagaras/IceNiagara/NS_22_PowerSmash_1_Ice.NS_22_PowerSmash_1_Ice" (+ (Transformation|GetActorLocation) (* (Transformation|GetActorForwardVector) (* (Variables|Default|GetIsSpawnNum) (Variables|Default|GetSpawnDistanceF)))) (Transformation|GetActorRotation) (select (< (- _spawnnum (Variables|Default|GetIsSpawnNum)) 5) (Math|Conversions|ToVector(Float) (Math|Float|MapRangeClamped (Math|Conversions|ToFloat(Integer) (- _spawnnum (Variables|Default|GetIsSpawnNum))) 5.0 1.0 1.1 1.6)) "1.000000,1.000000,1.000000"))
    (Math|Integer|IncrementInt (Variables|Default|GetIsSpawnNum)
      (:%20%20
        (Utilities|FlowControl|Delay (Variables|Default|GetTimeInterval))
        (goto _label)))))

(event EventBeginPlay)

(event Collision|EventActorBeginOverlap
  (params (OtherActor :type Actor%20Object%20Reference)))

(event EventTick
  (params (DeltaSeconds :type Float%20%28single-precision%29)))

(fn ConstructionScript)