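; Psy energy barrier actor that is toggled by key presses and destroys any actor that hits it.
; Keys 3 and 4 play or reverse a timeline driving the mesh's "Alpha Switcher" material parameter, while activating or deactivating the NSGround effect.
; Hits spawn a Niagara impact aligned to the surface normal and restart a sped-up Bounce timeline that animates a world-position-offset material parameter.
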(event OnComponentHit(SM_Barier)
  (params (HitComponent :type Primitive%20Component%20Object%20Reference) (OtherActor :type Actor%20Object%20Reference) (OtherComp :type Primitive%20Component%20Object%20Reference) (NormalImpulse :type Vector :default "0, 0, 0") (Hit :type Hit%20Result%20Structure%20%28by%20ref%29))
  (bind (_bblockinghit _binitialoverlap _time _distance _location _impactpoint _normal _impactnormal) (Collision|BreakHitResult Hit))
  (Actor|DestroyActor OtherActor)
  (Niagara|SpawnSystematLocation "/Game/Sci-Fi_All_In_One/VFX/NS_Impact_To_Psy_Shield.NS_Impact_To_Psy_Shield" _location (Math|Rotator|MakeRotfromX _impactnormal))
  (bind _newtrack_0 (Timeline|Bounce PlayFromStart)
    (:Update
      (Rendering|Material|SetScalarParameterValueonMaterials (Variables|Default|GetSM_Barier) "WPO Offset Bound" _newtrack_0))))

(event Custom|Hide%20Energy%20Barier
  (bind _newtrack_0 (Timeline|Barrier Reverse)
    (:Update
      (Rendering|Material|SetScalarParameterValueonMaterials (Variables|Default|GetSM_Barier) "Alpha Switcher" _newtrack_0))))

(event Custom|Show%20Energy%20Barier
  (bind _newtrack_0 (Timeline|Barrier Play)
    (:Update
      (Rendering|Material|SetScalarParameterValueonMaterials (Variables|Default|GetSM_Barier) "Alpha Switcher" _newtrack_0))))

(event EventBeginPlay
  (Components|Timeline|SetPlayRate (Variables|Default|GetBounce) 3.0))

(event Input|KeyboardEvents|3
  (params (Key :type Key%20Structure))
  (:Pressed
    (CallFunction|ShowEnergyBarier)
    (Components|Activation|Activate (Variables|Default|GetNS_Ground) false)))

(event Input|KeyboardEvents|4
  (params (Key :type Key%20Structure))
  (:Pressed
    (CallFunction|HideEnergyBarier)
    (Components|Activation|Deactivate (Variables|Default|GetNS_Ground))))

(fn ConstructionScript)