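; Holographic portal that teleports the third-person character to a linked PortalTarget and switches the camera to a newly spawned BP_Hyperportal.
; Entering the capsule hides the target portal to block an immediate return, then calls the character's own TeleportTo; leaving a capsule re-enables that portal.
; The construction script feeds PortalTexture through a dynamic material into the Niagara sphere as its 3D picture.
; The local TeleportTo is an unused template meant for copying into the character.
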(event OnComponentBeginOverlap(Capsule)
  (params (OverlappedComponent :type Primitive%20Component%20Object%20Reference) (OtherActor :type Actor%20Object%20Reference) (OtherComp :type Primitive%20Component%20Object%20Reference) (OtherBodyIndex :type Integer) (bFromSweep :type Boolean) (SweepResult :type Hit%20Result%20Structure%20%28by%20ref%29))
  (bind _portal_target (Variables|Default|GetPortal%20Target))
  (bind _asbp_third_person_character (Utilities|Casting|CastToBP_ThirdPersonCharacter OtherActor))
  (Variables|Default|SetPlayerOwn _asbp_third_person_character)
  (if (Variables|Default|GetCanTeleport)
    (CallFunction|HidePortal _portal_target)
    (Default|Teleportto (Variables|Default|GetPlayerOwn) (Transformation|GetWorldLocation (Variables|/Script/Engine.Actor|GetRootComponent _portal_target)) (Pawn|GetControlRotation (Game|GetPlayerController 0) :!class /Script/Engine.Controller))
    (bind _returnvalue (Game|SpawnActorfromClass "/Game/Sci-Fi_All_In_One/Blueprints/BP_Hyperportal.BP_Hyperportal_C" (Math|Transform|MakeTransform "0.000000,0.000000,1000.000000" "0, 0, 0" "1.000000,1.000000,1.000000") "AlwaysSpawn" "MultiplyWithRoot" 0 0))
    (bind _output_get (Variables|Default|SetPortal _returnvalue))
    (Game|Player|SetViewTargetwithBlend (Game|GetPlayerController 0) _output_get 0.0 "VTBlend_EaseInOut" 0.0 false)))

(event OnComponentEndOverlap(Capsule)
  (params (OverlappedComponent :type Primitive%20Component%20Object%20Reference) (OtherActor :type Actor%20Object%20Reference) (OtherComp :type Primitive%20Component%20Object%20Reference) (OtherBodyIndex :type Integer))
  (Utilities|Casting|CastToBP_ThirdPersonCharacter OtherActor)
  (CallFunction|ShowPortal))

(event Custom|Teleport%20To
  (params (Location :type Vector) (Rotation :type Rotator))
  ;[1 1 1] Teleport Function - Copy To You Character And Connect
)

(event Custom|Show%20Portal
  (Components|Activation|SetActive (Variables|Default|GetNS_Portal_Sphere) true true)
  (Variables|Default|SetCanTeleport true))

(event Custom|Hide%20Portal
  (Components|Activation|Deactivate (Variables|Default|GetNS_Portal_Sphere))
  (Variables|Default|SetCanTeleport false))

(event EventBeginPlay)

(fn ConstructionScript
  (bind _returnvalue (Rendering|Material|CreateDynamicMaterialInstance (Variables|Default|GetPortal%20Material) "None" "None" :!class /Script/Engine.KismetMaterialLibrary))
  (Rendering|Material|SetTextureParameterValue _returnvalue "3DPicTexture" (Variables|Default|GetPortal%20Texture))
  (Class|NiagaraComponent|SetVariableMaterial (Variables|Default|GetNS_Portal_Sphere) "3DPM" _returnvalue))