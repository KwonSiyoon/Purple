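; BP_Scaner is a scanner effect triggered by the E key, driven through the PC_Two_Side_Switch material parameter collection.
; Each scan plays a timeline that animates Radius and writes the player pawn's location to Player Position.
; It also sets HightLight to 1, then a second timeline drives that value.
; A DoOnce gates the input and is reset from the highlight timeline's Update, not on its completion.
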(event Input|KeyboardEvents|E
  (params (Key :type Key%20Structure :default "None"))
  ;[1 1 1] Change if need
  (:Pressed
    (Utilities|FlowControl|DoOnce false :!label _label
      (:Completed
        (Utilities|FlowControl|Sequence
          (:then_0
            (bind _newtrack_0 (Timeline|Scan PlayFromStart)
              (:Update
                (Rendering|Material|SetScalarParameterValue "/Game/Sci-Fi_All_In_One/Materials/Parameter_Collection/PC_Two_Side_Switch.PC_Two_Side_Switch" "Radius" _newtrack_0 :!class /Script/Engine.KismetMaterialLibrary))))
          (:then_1
            (Rendering|Material|SetScalarParameterValue "/Game/Sci-Fi_All_In_One/Materials/Parameter_Collection/PC_Two_Side_Switch.PC_Two_Side_Switch" "HightLight" 1.0 :!class /Script/Engine.KismetMaterialLibrary)
            ;[1 1 1] Change time if need
            (bind _newtrack_0_2 (Timeline|Off%20HL PlayFromStart)
              (:Update
                (Rendering|Material|SetScalarParameterValue "/Game/Sci-Fi_All_In_One/Materials/Parameter_Collection/PC_Two_Side_Switch.PC_Two_Side_Switch" "HightLight" _newtrack_0_2 :!class /Script/Engine.KismetMaterialLibrary)
                (goto _label Reset))))
          (:then_2
            (Rendering|Material|SetVectorParameterValue "/Game/Sci-Fi_All_In_One/Materials/Parameter_Collection/PC_Two_Side_Switch.PC_Two_Side_Switch" "Player Position" (Math|Conversions|ToLinearColor(Vector) (Transformation|GetActorLocation (Game|Player|GetPlayerPawn 0))) :!class /Script/Engine.KismetMaterialLibrary)))))))

(fn ConstructionScript)