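; Sci-fi energy gate Blueprint that animates on or off as actors enter and leave its trigger box.
; Overlap events toggle a FlipFlop that plays or reverses a timeline, driving the "On or Off" scalar in the PC_EDoor_Control Material Parameter Collection, a value shared globally.
; DoOnce gates entry until end overlap resets it.
; A delay after entry disables the door plane's collision, which is never re-enabled.
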(event OnComponentBeginOverlap(Box)
  (params (OverlappedComponent :type Primitive%20Component%20Object%20Reference) (OtherActor :type Actor%20Object%20Reference) (OtherComp :type Primitive%20Component%20Object%20Reference) (OtherBodyIndex :type Integer) (bFromSweep :type Boolean) (SweepResult :type Hit%20Result%20Structure%20%28by%20ref%29))
  (Utilities|FlowControl|DoOnce false
    (:Completed
      (CallFunction|EDoorAnimate)
      (Utilities|FlowControl|Delay 1.0)
      (Collision|SetCollisionEnabled (Variables|Default|GetSM_EDoor_Plane) "NoCollision"))))

(event OnComponentEndOverlap(Box)
  (params (OverlappedComponent :type Primitive%20Component%20Object%20Reference) (OtherActor :type Actor%20Object%20Reference) (OtherComp :type Primitive%20Component%20Object%20Reference) (OtherBodyIndex :type Integer))
  (CallFunction|EDoorAnimate)
  (Utilities|FlowControl|DoOnce false) ; enters at Reset
)

(event Custom|EDoor%20Animate
  (Utilities|FlowControl|FlipFlop
    (:A
      (bind _newtrack_0 (Timeline|EDoor%20On-Off Play)
        (:Update
          (Rendering|Material|SetScalarParameterValue "/Game/Sci-Fi_All_In_One/Materials/Parameter_Collection/PC_EDoor_Control.PC_EDoor_Control" "On or Off" _newtrack_0 :!class /Script/Engine.KismetMaterialLibrary))))
    (:B
      (Timeline|EDoor%20On-Off Reverse))))

(event EventBeginPlay)

(fn ConstructionScript)